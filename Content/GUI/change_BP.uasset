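; Actor with a widget component that acts as a gaze-activated restart control, tied to the VR game mode.
; Each tick it line-traces from the player camera along its forward vector against the widget.
; A hit plays a timeline that fills the change_widgit progress bar, and a miss reverses it.
; When the timeline finishes full, it calls RestartGame on VR_mode.
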(event `self.ReceiveTick`
  (params (DeltaSeconds :type "Float (single-precision)"))
  (bind _returnvalue (`GameplayStatics.GetPlayerCameraManager` 0))
  (bind _widget (`self.Widget`))
  (bind _returnvalue_2 (`self.K2_GetActorLocation` _returnvalue))
  (bind (_hitlocation _hitnormal _bonename _outhit _returnvalue_3) (`PrimitiveComponent.K2_LineTraceComponent` _widget _returnvalue_2 (+ _returnvalue_2 (* (`self.GetActorForwardVector` _returnvalue) 5000.0)) true false))
  (if _returnvalue_3
    (bind (_direction `_新規track_1`) (`Timeline|タイムライン_0` :!label _label)
      (:`Update`
        (bind _aschange_widgit (cast `/Game/GUI/change_widgit` (`WidgetComponent.GetUserWidgetObject` _widget)))
        (`ProgressBar.SetPercent` (`/Game/GUI/change_widgit.ProgressBar_37` _aschange_widgit) `_新規track_1`))
      (:`Finished`
        (if (>= `_新規track_1` 1.0)
          (bind _asvr_mode (cast `/Game/GUI/VR_mode` (`GameplayStatics.GetGameMode`)))
          (`GameMode.RestartGame` _asvr_mode))))
    (else
      (goto _label :!via `Reverse`))))

(fn `UserConstructionScript`)